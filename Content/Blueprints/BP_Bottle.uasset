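; BP_Bottle is a drinkable bottle that raises the VR pawn's hydration while it overlaps the bottle's DrinkCollision component.
; Overlap begin and end open and close a gate on Tick, which calls UpdateHydration with the overlapping actor.
; That function casts to VRPawn, adds a fixed amount to HYDRATION each frame, unclamped and independent of delta time, and prints the value.
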(event OnComponentBeginOverlap(DrinkCollision)
  (params (OverlappedComponent :type Primitive%20Component%20Object%20Reference) (OtherActor :type Actor%20Object%20Reference) (OtherComp :type Primitive%20Component%20Object%20Reference) (OtherBodyIndex :type Integer) (bFromSweep :type Boolean) (SweepResult :type Hit%20Result%20Structure%20%28by%20ref%29))
  (Utilities|FlowControl|Gate true) ; enters at Open
)

(event OnComponentEndOverlap(DrinkCollision)
  (params (OverlappedComponent :type Primitive%20Component%20Object%20Reference) (OtherActor :type Actor%20Object%20Reference) (OtherComp :type Primitive%20Component%20Object%20Reference) (OtherBodyIndex :type Integer))
  (Utilities|FlowControl|Gate true) ; enters at Close
)

(event EventBeginPlay)

(event Collision|EventActorBeginOverlap
  (params (OtherActor :type Actor%20Object%20Reference)))

(event EventTick
  (params (DeltaSeconds :type Float%20%28single-precision%29))
  (Utilities|FlowControl|Gate true
    (:Exit
      (CallFunction|UpdateHydration (stale OnComponentBeginOverlap(DrinkCollision) OtherActor)))))

(fn ConstructionScript)

(fn UpdateHydration
  (params (Pawn%20Reference :type Actor%20Object%20Reference))
  (bind _asvrpawn (Utilities|Casting|CastToVRPawn Pawn%20Reference))
  (bind _output_get (Variables|/Game/VRTemplate/Blueprints/VRPawn.VRPawn_C|SetHYDRATION _asvrpawn (+ (Variables|/Game/VRTemplate/Blueprints/VRPawn.VRPawn_C|GetHYDRATION _asvrpawn) 0.005)))
  (Development|PrintString (Utilities|String|ToString(Float) _output_get)))